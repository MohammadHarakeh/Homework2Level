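; MovingKiller is a hazard actor whose sphere slides back and forth and kills the player on touch.
; A timeline started on BeginPlay lerps the sphere's relative location along X, then reverses or replays on finish after a zero-length delay to ping-pong endlessly.
; When a ThirdPersonCharacter overlaps the sphere, it destroys that character and restarts the level through a console command.
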(event `self.Sphere1.OnComponentBeginOverlap`
  (params (OverlappedComponent :type "PrimitiveComponent Object Reference") (OtherActor :type "Actor Object Reference") (OtherComp :type "PrimitiveComponent Object Reference") (OtherBodyIndex :type Integer) (bFromSweep :type Boolean) (SweepResult :type "HitResult Structure (by ref)"))
  (bind _asthird_person_character (cast `/Game/ThirdPersonBP/Blueprints/ThirdPersonCharacter` OtherActor))
  (`self.K2_DestroyActor` _asthird_person_character)
  (`KismetSystemLibrary.ExecuteConsoleCommand` "RestartLevel" null))

(event `self.ReceiveBeginPlay`
  (bind _timeline_0 (`self.Timeline_0`))
  (bind (_direction _newtrack_0) (`Timeline|Timeline_0` :!via `PlayFromStart`)
    (:`Update`
      (`SceneComponent.K2_SetRelativeLocation` (`self.Sphere1`) (`KismetMathLibrary.VLerp` (0.0 0.0 0.0) (2200.0 0.0 0.0) _newtrack_0) false false))
    (:`Finished`
      (`KismetSystemLibrary.Delay` 0.0)
      (if (`|EnumEquality` _direction "Forward")
        (`TimelineComponent.ReverseFromEnd` _timeline_0)
        (else
          (`TimelineComponent.PlayFromStart` _timeline_0))))))

(fn `UserConstructionScript`)